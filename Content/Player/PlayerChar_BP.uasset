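; Player character Blueprint that toggles a crafting menu and carries Health, Hunger and Stamina stats.
; The CraftMenu input drives a FlipFlop that creates and shows a new crafting widget with mouse cursor and Game-and-UI input, then removes it and restores game-only input and viewport focus.
; Tick prints the three stats to screen as a testing aid; nothing in these graphs changes them.
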(event `self.ReceiveTick`
  (params (DeltaSeconds :type "Float (single-precision)"))
  ; Testing: print value of health, hunger, and stamina
  (`KismetSystemLibrary.PrintString` (`KismetStringLibrary.Concat_StrStr` "Stamina: " (`KismetStringLibrary.Conv_DoubleToString` (`self.Stamina`)) " \n") true true (struct :`R` 1.0 :`G` 0.50199 :`A` 1.0))
  (`KismetSystemLibrary.PrintString` (`KismetStringLibrary.Concat_StrStr` "Hunger: " (`KismetStringLibrary.Conv_DoubleToString` (`self.Hunger`))) true true (struct :`R` 0.15109 :`G` 0.495185 :`B` 1.0 :`A` 1.0))
  (`KismetSystemLibrary.PrintString` (`KismetStringLibrary.Concat_StrStr` "Health: " (`KismetStringLibrary.Conv_DoubleToString` (`self.Health`))) true true (struct :`R` 0.01574 :`G` 1.0 :`A` 1.0)))

(event `InputAction|CraftMenu`
  (params (Key :type "Key Structure"))
  (bind _returnvalue (`GameplayStatics.GetPlayerController` 0))
  ; Opening Craft Menu
  (:`Pressed`
    (`/Engine/EditorBlueprintResources/StandardMacros.FlipFlop`
      (:`A`
        (bind _returnvalue_2 (`|CreateWidget` "/Game/Widgets/Crafting_W.Crafting_W_C"))
        (`UserWidget.AddToViewport` _returnvalue_2 0)
        (set `PlayerController.bShowMouseCursor` true _returnvalue)
        (`WidgetBlueprintLibrary.SetInputMode_GameAndUIEx` _returnvalue _returnvalue_2))
      (:`B`
        (`Widget.RemoveFromParent` _returnvalue_2)
        (set `PlayerController.bShowMouseCursor` false _returnvalue)
        (`WidgetBlueprintLibrary.SetInputMode_GameOnly` _returnvalue)
        (`WidgetBlueprintLibrary.SetFocusToGameViewport`)))))

(fn `UserConstructionScript`)